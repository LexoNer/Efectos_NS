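; Water area actor that shows a Niagara effect while the third-person character moves inside its Box volume.
; Box overlap begin and end set a flag for the player being inside and toggle the effect's visibility.
; While the flag is set, Tick moves the Niagara component to the character mesh location and hides it whenever the character's velocity is zero.
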(event OnComponentBeginOverlap(Box)
  (params (OverlappedComponent :type Primitive%20Component%20Object%20Reference) (OtherActor :type Actor%20Object%20Reference) (OtherComp :type Primitive%20Component%20Object%20Reference) (OtherBodyIndex :type Integer) (bFromSweep :type Boolean) (SweepResult :type Hit%20Result%20Structure%20%28by%20ref%29))
  (bind _asbp_third_person_character (Utilities|Casting|CastToBP_ThirdPersonCharacter OtherActor))
  (Development|SetHiddeninGame (Variables|Default|GetNiagara) false false)
  (Variables|Default|SetPos true))

(event OnComponentEndOverlap(Box)
  (params (OverlappedComponent :type Primitive%20Component%20Object%20Reference) (OtherActor :type Actor%20Object%20Reference) (OtherComp :type Primitive%20Component%20Object%20Reference) (OtherBodyIndex :type Integer))
  (Utilities|Casting|CastToBP_ThirdPersonCharacter OtherActor)
  (Development|SetHiddeninGame (Variables|Default|GetNiagara) true false)
  (Variables|Default|SetPos false))

(event EventBeginPlay
  (bind _asbp_third_person_character (Utilities|Casting|CastToBP_ThirdPersonCharacter (Game|GetPlayerCharacter 0)))
  (Variables|Default|SetAs%20BP%20Third%20Person%20Character _asbp_third_person_character)
  (Development|SetHiddeninGame (Variables|Default|GetNiagara) true false))

(event EventTick
  (params (DeltaSeconds :type Float%20%28single-precision%29))
  (bind _niagara (Variables|Default|GetNiagara))
  (bind _as_bp_third_person_character (Variables|Default|GetAs%20BP%20Third%20Person%20Character))
  (if (Variables|Default|GetPos)
    (if (> (Math|Vector|VectorLength (Pawn|Components|CharacterMovement|GetLastUpdateVelocity (Variables|/Script/Engine.Character|GetCharacterMovement _as_bp_third_person_character))) 0.0)
      (Development|SetHiddeninGame _niagara false false)
      (Transformation|SetWorldLocation (Variables|Default|GetNiagara) (Transformation|GetWorldLocation (Variables|/Script/Engine.Character|GetMesh _as_bp_third_person_character)) false false)
      (else
        (Development|SetHiddeninGame _niagara true false)))))

(fn ConstructionScript)